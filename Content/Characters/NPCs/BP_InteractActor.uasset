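; BP_InteractActor is an NPC interaction actor that displays its NpcText lines in an on-screen dialogue box.
; The Dialogue event removes an existing box and resets, or creates WBP_DialogueBox, adds it to the viewport and calls TalkTo.
; Behind a DoOnce gate, TalkTo passes the lines to the widget, reveals it, then either removes it or zeroes its row based on array length.
; ResetDialogue only reopens that gate.
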(event Custom|ResetDialogue
  (Utilities|FlowControl|DoOnce false) ; enters at Reset
)

(event Custom|TalkTo
  (Utilities|FlowControl|DoOnce false ; Reads lines of dialogue from the\nNpcText array
    (:Completed
      (Variables|/Game/WBP_DialogueBox.WBP_DialogueBox_C|SetText (Variables|Default|GetDialogueBox) (Variables|Default|GetNpcText))
      (Widget|SetVisibility (Variables|/Game/WBP_DialogueBox.WBP_DialogueBox_C|GetTextBlock_0 (Variables|Default|GetDialogueBox)) "Visible") ; Shows the dialogue box
      (if (> (+ (Variables|/Game/WBP_DialogueBox.WBP_DialogueBox_C|GetTextRow (Variables|Default|GetDialogueBox)) 1) (- (Utilities|Array|Length (Variables|Default|GetNpcText)) 1))
        (Widget|RemovefromParent (Variables|Default|GetDialogueBox)) ; Removes widget from\nplayer screen if all \ndialogue is exhausted
        (CallFunction|Resetdialogue) ; Resets the dialogue
        (else
          (Variables|/Game/WBP_DialogueBox.WBP_DialogueBox_C|SetTextRow (Variables|Default|GetDialogueBox) 0)
          (CallFunction|Resetdialogue))))))

(event EventBeginPlay)

(event Collision|EventActorBeginOverlap
  (params (OtherActor :type Actor%20Object%20Reference)))

(event EventTick
  (params (DeltaSeconds :type Float%20%28single-precision%29)))

(event EventDialogue
  (Utilities|IsValid (Variables|Default|GetDialogueBox)
    (:Is%20Valid
      (Widget|RemovefromParent (Variables|Default|GetDialogueBox))
      (CallFunction|ResetDialogue))
    (:Is%20Not%20Valid
      (bind _returnvalue (UserInterface|CreateWidget "/Game/WBP_DialogueBox.WBP_DialogueBox_C" (Game|GetPlayerController 0))) ; Makes sure that WBP_DialogueBox is created
      (bind _output_get (Variables|Default|SetDialogueBox _returnvalue))
      (UserInterface|Viewport|AddtoViewport _output_get 0) ; Adds the dialogue box to \nplayer's screen
      (CallFunction|Talkto))))

(fn ConstructionScript)